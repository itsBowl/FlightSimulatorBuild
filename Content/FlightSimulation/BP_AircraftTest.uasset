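; Test aircraft pawn that maps player flight controls to throttle, roll, pitch, yaw and flap input variables.
; On possession by a player, it adds the default flight Enhanced Input context.
; Roll, pitch and yaw store scaled axis values, while throttle and flaps toggle once per press through DoOnce and FlipFlop.
; Tick prints pitch, yaw, roll and throttle for debugging; no flight physics is computed in this graph.
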(event Input|EnhancedActionEvents|EnhancedInputActionIA_Throttle
  (params (ActionValue :type Boolean) (ElapsedSeconds :type Float%20%28double-precision%29) (TriggeredSeconds :type Float%20%28double-precision%29) (InputAction :type Input%20Action%20Object%20Reference :default "/Game/FlightSimulation/Input/IA_Throttle.IA_Throttle"))
  (:Triggered
    (Utilities|FlowControl|DoOnce false :!label _label
      (:Completed
        (Utilities|FlowControl|FlipFlop
          (:A
            (Variables|Default|SetthrottleInput 1.0))
          (:B
            (Variables|Default|SetthrottleInput 0.0))))))
  (:Completed
    (goto _label Reset)))

(event Input|EnhancedActionEvents|EnhancedInputActionIA_Roll
  (params (ActionValue :type Float%20%28double-precision%29) (ElapsedSeconds :type Float%20%28double-precision%29) (TriggeredSeconds :type Float%20%28double-precision%29) (InputAction :type Input%20Action%20Object%20Reference :default "/Game/FlightSimulation/Input/IA_Roll.IA_Roll"))
  (:Triggered
    (Variables|Default|SetrollInput (* ActionValue 0.2) :!label _label))
  (:Canceled
    (goto _label))
  (:Completed
    (goto _label)))

(event Input|EnhancedActionEvents|EnhancedInputActionIA_Pitch
  (params (ActionValue :type Float%20%28double-precision%29) (ElapsedSeconds :type Float%20%28double-precision%29) (TriggeredSeconds :type Float%20%28double-precision%29) (InputAction :type Input%20Action%20Object%20Reference :default "/Game/FlightSimulation/Input/IA_Pitch.IA_Pitch"))
  (:Triggered
    (Variables|Default|SetpitchInput (* ActionValue 0.3) :!label _label))
  (:Canceled
    (goto _label))
  (:Completed
    (goto _label)))

(event Input|EnhancedActionEvents|EnhancedInputActionIA_Yaw
  (params (ActionValue :type Float%20%28double-precision%29) (ElapsedSeconds :type Float%20%28double-precision%29) (TriggeredSeconds :type Float%20%28double-precision%29) (InputAction :type Input%20Action%20Object%20Reference :default "/Game/FlightSimulation/Input/IA_Yaw.IA_Yaw"))
  (:Triggered
    (Variables|Default|SetyawInput (* ActionValue 0.5) :!label _label))
  (:Canceled
    (goto _label))
  (:Completed
    (goto _label)))

(event Input|EnhancedActionEvents|EnhancedInputActionIA_Flaps
  (params (ActionValue :type Boolean) (ElapsedSeconds :type Float%20%28double-precision%29) (TriggeredSeconds :type Float%20%28double-precision%29) (InputAction :type Input%20Action%20Object%20Reference :default "/Game/FlightSimulation/Input/IA_Flaps.IA_Flaps"))
  (:Triggered
    (Utilities|FlowControl|DoOnce false :!label _label
      (:Completed
        (Utilities|FlowControl|FlipFlop
          (:A
            (Variables|Default|SetflapInput 0.3))
          (:B
            (Variables|Default|SetflapInput 0.0))))))
  (:Completed
    (goto _label Reset)))

(event EventPossessed
  (params (NewController :type Controller%20Object%20Reference))
  (bind _asplayer_controller (Utilities|Casting|CastToPlayerController NewController))
  (Input|AddMappingContext (PlayerController|LocalPlayerSubsystems|GetEnhancedInputLocalPlayerSubsystem _asplayer_controller) "/Game/FlightSimulation/Input/IMC_FlightDefault.IMC_FlightDefault" 0 "(bIgnoreAllPressedKeysUntilRelease=True,bForceImmediately=False,bNotifyUserSettings=False)"))

(event EventTick
  (params (DeltaSeconds :type Float%20%28single-precision%29))
  (Development|PrintString (Utilities|String|Append "Pitch: " (Utilities|String|ToString(Float) (Variables|Default|GetpitchInput)) " Yaw: " (Utilities|String|ToString(Float) (Variables|Default|GetyawInput)) " Roll: " (Utilities|String|ToString(Float) (Variables|Default|GetrollInput)) " ThrotleState: " (Utilities|String|ToString(Float) (Variables|Default|GetthrottleInput))) true true "(R=0.000000,G=0.660000,B=1.000000,A=1.000000)" DeltaSeconds))

(fn ConstructionScript)